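; A moving platform Blueprint that makes a single one-way trip from its starting position to the location of its TargetBox component.
; BeginPlay caches both endpoints, and any overlap with the Box component starts the motion.
; Tick advances an alpha over about five seconds, lerps the actor's location without sweep, and stops permanently once alpha exceeds one.
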(event `self.ReceiveBeginPlay`
  (set `self.OriginalLoc` (`self.K2_GetActorLocation`))
  (set `self.TargetLoc` (`SceneComponent.K2_GetComponentLocation` (`self.TargetBox`))))

(event `self.ReceiveActorBeginOverlap`
  (params (OtherActor :type "Actor Object Reference")))

(event `self.ReceiveTick`
  (params (DeltaSeconds :type "Float (single-precision)"))
  (if (`self.ReachEnd`)
    _
    (elif (`self.Moving`)
      (bind _output_get (set `self.CurAlpha` (+ (/ DeltaSeconds 5.0) (`self.CurAlpha`))))
      (`self.K2_SetActorLocation` (`KismetMathLibrary.VLerp` (`self.OriginalLoc`) (`self.TargetLoc`) _output_get))
      (`/Engine/EditorBlueprintResources/StandardMacros.CompareFloat` (`self.CurAlpha`) 1.0
        (:`>`
          (set `self.ReachEnd` true))))))

(event `self.Box.OnComponentBeginOverlap`
  (params (OverlappedComponent :type "PrimitiveComponent Object Reference") (OtherActor :type "Actor Object Reference") (OtherComp :type "PrimitiveComponent Object Reference") (OtherBodyIndex :type Integer) (bFromSweep :type Boolean) (SweepResult :type "HitResult Structure (by ref)"))
  (set `self.Moving` true))

(fn `UserConstructionScript`)