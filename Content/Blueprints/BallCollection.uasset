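; BallCollection is a component-style Blueprint that tracks rings left to collect and gates the goal for the player ball.
; AddRing raises RingCount, while CollectRing lowers it and plays a coin sound at the owner's location.
; CanCollectGoal returns true once the count is zero or below.
; CollectGoal casts the owner to PlayerBall and activates its WinConfetti, without checking that condition itself.
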(fn `AddRing`
  (set `self.RingCount` (+ (`self.RingCount`) 1)))

(fn `CanCollectGoal`
  (returns (CanCollect :type Boolean))
  (return (<= (`self.RingCount`) 0)))

(fn `CollectGoal`
  (bind _asplayer_ball (cast `/Game/Blueprints/PlayerBall` (`self.GetOwner`)))
  (`self.SetActive` (`/Game/Blueprints/PlayerBall.WinConfetti` _asplayer_ball) true false))

(fn `CollectRing`
  (set `self.RingCount` (+ (`self.RingCount`) -1))
  (`GameplayStatics.PlaySoundAtLocation` "/Game/Sounds/Mario_Coin_Sound_-_Sound_Effect__HD_.Mario_Coin_Sound_-_Sound_Effect__HD_" (`Actor.K2_GetActorLocation` (`self.GetOwner`)) (struct) 0.5 1.0 0.35 null null null null))