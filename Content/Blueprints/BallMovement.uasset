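; BallMovement is a component that moves and jumps its owning PlayerBall by applying physics forces to its Sphere.
; MoveY and MoveX mask the forward and right arrows' directions to world X and Y respectively, while Jump follows the jump arrow.
; All three scale force by the sphere's mass, apply it at the forward arrow's location, and print debug values.
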(fn `Jump`
  (bind _asplayer_ball (cast `/Game/Blueprints/PlayerBall` (`self.GetOwner`)))
  (bind _sphere (`/Game/Blueprints/PlayerBall.Sphere` _asplayer_ball))
  (bind _returnvalue (`SceneComponent.K2_GetComponentLocation` (`/Game/Blueprints/PlayerBall.ForwardArrow` _asplayer_ball)))
  (`PrimitiveComponent.AddForceAtLocation` _sphere (* (`SceneComponent.GetForwardVector` (`/Game/Blueprints/PlayerBall.JumpArrow` _asplayer_ball)) (`self.JumpForce`) (`PrimitiveComponent.GetMass` _sphere)) _returnvalue "None")
  (`KismetSystemLibrary.PrintString` (`KismetStringLibrary.Conv_VectorToString` _returnvalue)))

(fn `MoveX`
  (params (Value :type "Float (double-precision)"))
  (bind _asplayer_ball (cast `/Game/Blueprints/PlayerBall` (`self.GetOwner`)))
  (bind _sphere (`/Game/Blueprints/PlayerBall.Sphere` _asplayer_ball))
  (bind _returnvalue (* (`KismetMathLibrary.MakeVector` 0.0 Value) (`SceneComponent.GetForwardVector` (`/Game/Blueprints/PlayerBall.RightArrow` _asplayer_ball)) (`self.MoveForce`) (`PrimitiveComponent.GetMass` _sphere)))
  (`PrimitiveComponent.AddForceAtLocation` _sphere _returnvalue (`SceneComponent.K2_GetComponentLocation` (`/Game/Blueprints/PlayerBall.ForwardArrow` _asplayer_ball)) "None")
  (`KismetSystemLibrary.PrintString` (`KismetStringLibrary.Conv_VectorToString` _returnvalue)))

(fn `MoveY`
  (params (Value :type "Float (double-precision)"))
  (bind _asplayer_ball (cast `/Game/Blueprints/PlayerBall` (`self.GetOwner`)))
  (bind _sphere (`/Game/Blueprints/PlayerBall.Sphere` _asplayer_ball))
  (bind _forwardarrow (`/Game/Blueprints/PlayerBall.ForwardArrow` _asplayer_ball))
  (bind _returnvalue (* (`KismetMathLibrary.MakeVector` Value) (`SceneComponent.GetForwardVector` _forwardarrow) (`self.MoveForce`) (`PrimitiveComponent.GetMass` _sphere)))
  (`PrimitiveComponent.AddForceAtLocation` _sphere _returnvalue (`SceneComponent.K2_GetComponentLocation` _forwardarrow) "None")
  (`KismetSystemLibrary.PrintString` (`KismetStringLibrary.Conv_VectorToString` _returnvalue)))